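; Maguro sushi recovery pickup that BP_UQ5_Player collects by contact.
; A mesh hit adds an audio component, calls GetRecoveryItem on the first BP_UQ5_Player found and destroys the sushi, guarded by DoOnce.
; The "Player" tag check on the hit actor's owner has empty branches, so it filters nothing.
; A work-in-progress floating effect starts at BeginPlay, adding a timeline-driven local Z offset each update.
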(event OnComponentHit(StaticMeshComponent)
  (params (HitComponent :type Primitive%20Component%20Object%20Reference) (OtherActor :type Actor%20Object%20Reference) (OtherComp :type Primitive%20Component%20Object%20Reference) (NormalImpulse :type Vector :default "0, 0, 0") (Hit :type Hit%20Result%20Structure%20%28by%20ref%29))
  ;[1 1 1] 触れたアクタのタグがPlayerなら、BP_UQ5_PlayerにGet_Recavary_Itemを送る
  (if (Actor|ActorHasTag (Components|GetOwner OtherActor) "Player")
    _
    (else
      _))
  (Utilities|FlowControl|DoOnce false
    (:Completed
      (AddComponent|AddAudioComponent false)
      (bind _returnvalue (Actor|GetActorOfClass "/Game/UnrealQuest5/Blueprints/BP_UQ5_Player.BP_UQ5_Player_C"))
      (Default|GetRecoveryItem _returnvalue)
      (Actor|DestroyActor))))

(event EventBeginPlay
  ;[1 1 1] ふわふわ浮かせる処理　作成中　https://unrealengine.hatenablog.com/entry/2014/08/25/234215
  (bind _movevalue (Timeline|タイムライン Play)
    (:Update
      (Transformation|AddActorLocalOffset (Math|Vector|MakeVector 0.0 0.0 _movevalue) false false))))

(fn ConstructionScript)