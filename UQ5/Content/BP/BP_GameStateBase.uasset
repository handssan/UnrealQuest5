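; Game state that handles the stage's win/lose display and player HP readout.
; BeginPlay resets the kill count against a fixed enemy total and adds the Win, Lose, HP label and HP value widgets to the viewport.
; Enemydead shows Win once kills reach the total, and Player_Lose shows Lose.
; GetItem copies BP_UQ5_Player's truncated HP into the value widget.
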(event Custom|GetItem
  (bind _returnvalue (Actor|GetActorOfClass "/Game/UnrealQuest5/Blueprints/BP_UQ5_Player.BP_UQ5_Player_C"))
  (Variables|/Game/UI/WBP_PlayerHPValue.WBP_PlayerHPValue_C|SetUI_Text (Variables|Default|GetVar_Wdget_HPValue) (Utilities|Text|ToText(Integer) (Math|Float|Truncate (Variables|/Game/UnrealQuest5/Blueprints/BP_UQ5_Player.BP_UQ5_Player_C|GetHP _returnvalue)))))

(event Custom|Enemydead
  ;[1 1 1] 敵を全部倒したかの判定⇒「Ｗｉｎ」の表示をオンにする
  (if (>= (Variables|Default|GetKillCount) (Variables|Default|GetEnemyTotal))
    (Widget|SetVisibility (Variables|Default|GetVar_Widget_Win) "Visible")))

(event Custom|Player_Lose
  ;[1 1 1] プレイヤーが倒されたかの判定⇒「ＬＯＳＥ」の表示をオンにする
  (Widget|SetVisibility (Variables|Default|GetVar_Widget_LOSE) "Visible"))

(event EventBeginPlay
  ;[1 1 1] ステージInit　変数の初期化・各widgetを配置
  (Variables|Default|SetKillCount 0)
  (Variables|Default|SetEnemyTotal 4)
  ;;[1 1 1] 「WIN」のテキストを配置
  (bind _returnvalue (UserInterface|CreateWidget "/Game/UI/WBP_Text_Win.WBP_Text_Win_C"))
  (bind _output_get (Variables|Default|SetVar_Widget_Win _returnvalue))
  (UserInterface|Viewport|AddtoViewport _output_get 0)
  ;;[1 1 1] 「LOSE」のテキストを配置
  (bind _returnvalue_2 (UserInterface|CreateWidget "/Game/UI/WBP_Text_LOSE.WBP_Text_LOSE_C"))
  (bind _output_get_2 (Variables|Default|SetVar_Widget_LOSE _returnvalue_2))
  (UserInterface|Viewport|AddtoViewport _output_get_2 0)
  ;;[1 1 1] 「HP」のテキストを配置
  (bind _returnvalue_3 (UserInterface|CreateWidget "/Game/UI/WBP_PlayerHP.WBP_PlayerHP_C"))
  (bind _output_get_3 (Variables|Default|SetVar_Widget_HP _returnvalue_3))
  (UserInterface|Viewport|AddtoViewport _output_get_3 0)
  ;;[1 1 1] 「HPの数値」のテキストを配置
  (bind _returnvalue_4 (UserInterface|CreateWidget "/Game/UI/WBP_PlayerHPValue.WBP_PlayerHPValue_C"))
  (bind _output_get_4 (Variables|Default|SetVar_Wdget_HPValue _returnvalue_4))
  (UserInterface|Viewport|AddtoViewport _output_get_4 0))

(fn ConstructionScript)