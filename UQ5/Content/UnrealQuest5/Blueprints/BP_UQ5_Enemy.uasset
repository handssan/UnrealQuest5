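; Enemy character for UnrealQuest5 that plays an attack montage, takes damage and dies, with its child actor weapon owned by itself to avoid self-damage.
; AnyDamage lowers EnemyHP and plays a hit montage while HP remains.
; At zero HP, a one-time sequence plays a montage, switches the mesh to ragdoll just before it ends, then updates BP_GameStateBase's kill count, calls Enemydead, spawns fire and destroys the actor.
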(event Custom|Attack
  ;[1 0 0 0.5] 攻撃
  (Animation|PlayAnimMontage "/Game/UnrealQuest5/Characters/Mannequins/Animations/UQ5/AM_Attack01.AM_Attack01" 1.0 "None"))

(event Game|Damage|EventAnyDamage
  (params (Damage :type Float%20%28single-precision%29) (DamageType :type Damage%20Type%20Object%20Reference) (InstigatedBy :type Controller%20Object%20Reference) (DamageCauser :type Actor%20Object%20Reference))
  (bind _mesh (Variables|Character|GetMesh))
  ;[1 1 1] 攻撃を受けた場合の処理
  (Development|PrintString (Utilities|GetDisplayName DamageCauser))
  (bind _output_get (Variables|Default|SetEnemyHP (- (Variables|Default|GetEnemyHP) Damage)))
  (AddComponent|AddAudioComponent false)
  (if (> _output_get 0.0)
    (Development|PrintString "Alive")
    ;;[1 1 1] HPがまだ残っている→ダメージ処理
    (Animation|PlayAnimMontage "/Game/UnrealQuest5/Characters/Mannequins/Animations/UQ5/AM_Damaged_Montage.AM_Damaged_Montage" 1.0 "None")
    (else
      (Development|PrintString "Dead")
      (Utilities|FlowControl|DoOnce false
        (:Completed
          ;;[1 1 1] 死んだ時
          (bind _returnvalue (Animation|PlayAnimMontage "/Game/UnrealQuest5/Characters/Mannequins/Animations/UQ5/AM_GotParried_Montage.AM_GotParried_Montage" 1.0 "None"))
          (AddComponent|AddAudioComponent false)
          (Development|PrintString (Utilities|String|ToString(Float) (Variables|Default|GetEnemyHP)))
          (Utilities|FlowControl|Delay (- _returnvalue 0.27))
          (Variables|/Script/Engine.SkeletalMeshComponent|SetbPauseAnims (Variables|Character|GetMesh) false)
          (Pawn|Components|CharacterMovement|DisableMovement (Variables|Character|GetCharacterMovement))
          ;[1 1 1] 刀に触れた時BP_KatanaからDamageを受け取りラグドール化する
          (Collision|SetCollisionProfileName _mesh "Ragdoll" true :!class /Script/Engine.PrimitiveComponent)
          (Physics|SetSimulatePhysics _mesh true)
          (Utilities|FlowControl|Delay 3.0)
          (Effects|SpawnEmitteratLocation 0 (Transformation|GetActorLocation)) ; あとで適当なエフェクト（死亡時）を設定する
          ;[1 1 1] 他のＢＰを参照する時の参考(このＢＰからGameStateBaseにEnemydead
          (bind _asbp_game_state_base (Utilities|Casting|CastToBP_GameStateBase (Game|GetGameState)))
          (Variables|/Game/BP/BP_GameStateBase.BP_GameStateBase_C|SetKillCount _asbp_game_state_base (+ (Variables|/Game/BP/BP_GameStateBase.BP_GameStateBase_C|GetKillCount _asbp_game_state_base) 1))
          (Default|Enemydead _asbp_game_state_base)
          (Effects|SpawnEmitteratLocation "/Game/LowpolyStyle/Asia/Particles/PS_Fire.PS_Fire" (Transformation|GetActorLocation))
          (Actor|DestroyActor))))))

(event EventBeginPlay
  ;[1 1 1] 剣で自分がダメージを受けないようにする
  (Development|PrintString (Utilities|String|ToString(Float) (Variables|Default|GetEnemyHP)))
  (Actor|SetOwner (Variables|/Script/Engine.ChildActorComponent|GetChildActor (Variables|Default|GetChildActor)) self))

(fn ConstructionScript)